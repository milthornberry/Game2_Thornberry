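; BP_NPC is a dialogue NPC that shows voiced lines from DT_Dialogue when the third-person character is in range.
; Entering its sphere registers the NPC on the player and shows a W_NPDialogue widget.
; Each NextLine call reads the next table row by index, setting text and audio, with justification set only for NPC-spoken lines.
; Leaving or passing the last row clears references, hides the widget and resets the index to zero.
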(event `self.ReceiveBeginPlay`
  (bind _returnvalue (`|CreateWidget` "/Game/DialogueSystem/W_NPDialogue.W_NPDialogue_C"))
  (set `self.W Dialogue` _returnvalue)
  (set `self.NextLineIndex` (`self.StartingLineIndex`)))

(event `self.Sphere.OnComponentBeginOverlap`
  (params (OverlappedComponent :type "PrimitiveComponent Object Reference") (OtherActor :type "Actor Object Reference") (OtherComp :type "PrimitiveComponent Object Reference") (OtherBodyIndex :type Integer) (bFromSweep :type Boolean) (SweepResult :type "HitResult Structure (by ref)"))
  (bind _asbp_third_person_character (cast `/Game/ThirdPerson/Blueprints/BP_ThirdPersonCharacter` OtherActor))
  (bind _output_get (set `self.Player` _asbp_third_person_character))
  (set `/Game/ThirdPerson/Blueprints/BP_ThirdPersonCharacter.NPC` self _output_get)
  (`UserWidget.AddToViewport` (`self.W Dialogue`) 0))

(event `self.Sphere.OnComponentEndOverlap`
  (params (OverlappedComponent :type "PrimitiveComponent Object Reference") (OtherActor :type "Actor Object Reference") (OtherComp :type "PrimitiveComponent Object Reference") (OtherBodyIndex :type Integer))
  (cast `/Game/ThirdPerson/Blueprints/BP_ThirdPersonCharacter` OtherActor)
  (`self.End Dialogue`))

(event `End Dialogue`
  (set `/Game/ThirdPerson/Blueprints/BP_ThirdPersonCharacter.NPC` null (`self.Player`)) ; set npc to nothing
  (set `self.Player` null) ; Set player to nothing
  (`Widget.RemoveFromParent` (`self.W Dialogue`)) ; Hide the dialogue
  (set `self.NextLineIndex` 0))

(event `Next Line`
  (bind _audio (`self.Audio`))
  (bind _outrownames (`DataTableFunctionLibrary.GetDataTableRowNames` "/Game/DialogueSystem/DT_Dialogue.DT_Dialogue"))
  (if (> (`self.NextLineIndex`) (`KismetArrayLibrary.Array_LastIndex` _outrownames))
    (`self.End Dialogue`)
    (else
      (bind _returnvalue (`|GetDataTableRow` "/Game/DialogueSystem/DT_Dialogue.DT_Dialogue" (`|GetArrayItem` _outrownames (`self.NextLineIndex`)))
        (:`then`
          (`TextBlock.SetText` (`/Game/DialogueSystem/W_NPDialogue.TextBlock_0` (`self.W Dialogue`)) (`KismetTextLibrary.Conv_StringToText` (break `/Game/DialogueSystem/S_NPC_Dialogue` _returnvalue)))
          (`/Engine/EditorBlueprintResources/StandardMacros.IncrementInt` (`self.NextLineIndex`) ; Increment int
            (:`  `
              (`AudioComponent.SetSound` _audio (`.VoicedLine_6_14BCFA4448CC30F36F786EA929C7BC7E` (break `/Game/DialogueSystem/S_NPC_Dialogue` _returnvalue)))
              (`AudioComponent.Play` _audio 0.0)
              (switch `/Game/DialogueSystem/E_Speaker` (`.Speaker_8_86F4ED3B4BD67CCFF4E7C48FA4437D73` (break `/Game/DialogueSystem/S_NPC_Dialogue` _returnvalue))
                (:`NewEnumerator0`
                  (set `TextLayoutWidget.Justification` (select `/Game/DialogueSystem/E_Speaker` (`.Speaker_8_86F4ED3B4BD67CCFF4E7C48FA4437D73` (break `/Game/DialogueSystem/S_NPC_Dialogue` _returnvalue)) :`NewEnumerator0` "Left" :`NewEnumerator1` "Right" :!type "ETextJustify Enum") (`/Game/DialogueSystem/W_NPDialogue.TextBlock_0` (`self.W Dialogue`))))))))))))

(fn `UserConstructionScript`)