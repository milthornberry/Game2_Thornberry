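; BP_Cauldron is a crafting station actor that turns the player's collected ingredients into a potion.
; When the third-person character overlaps its collision, it checks that no potion has been made and that both ingredient counts meet a threshold.
; On success it spawns BP_Potion at a hardcoded world location, resets the character's inventory and sets its MadePotion flag.
; Each outcome is reported with a printed message.
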(event `self.ReceiveBeginPlay`
  (bind _asbp_third_person_character (cast `/Game/ThirdPerson/Blueprints/BP_ThirdPersonCharacter` (`GameplayStatics.GetPlayerCharacter` 0)))
  (set `self.PlayerReference` _asbp_third_person_character))

(event `self.Collision.OnComponentBeginOverlap`
  (params (OverlappedComponent :type "PrimitiveComponent Object Reference") (OtherActor :type "Actor Object Reference") (OtherComp :type "PrimitiveComponent Object Reference") (OtherBodyIndex :type Integer) (bFromSweep :type Boolean) (SweepResult :type "HitResult Structure (by ref)"))
  (bind _asbp_third_person_character (cast `/Game/ThirdPerson/Blueprints/BP_ThirdPersonCharacter` OtherActor))
  (if true
    (if (`/Game/ThirdPerson/Blueprints/BP_ThirdPersonCharacter.MadePotion` _asbp_third_person_character)
      (`KismetSystemLibrary.PrintString` "Potion already made")
      (elif (and (>= (`/Game/ThirdPerson/Blueprints/BP_ThirdPersonCharacter.Ingredient1` _asbp_third_person_character) 3) (>= (`/Game/ThirdPerson/Blueprints/BP_ThirdPersonCharacter.Ingredient2` _asbp_third_person_character) 3))
        (`KismetSystemLibrary.PrintString` "making potion")
        (`self.CreatePotion`)
        (`/Game/ThirdPerson/Blueprints/BP_ThirdPersonCharacter.Reset Inventory` _asbp_third_person_character)
        (set `/Game/ThirdPerson/Blueprints/BP_ThirdPersonCharacter.MadePotion` true _asbp_third_person_character)
        (else
          (`KismetSystemLibrary.PrintString` "Need more ingredients"))))))

(event `CreatePotion`
  (`|SpawnActorFromClass` "/Game/Content/BP_Potion.BP_Potion_C" (`KismetMathLibrary.MakeTransform` (-1305.0 1545.0 225.0)) "Undefined" "MultiplyWithRoot" null null))

(fn `UserConstructionScript`)